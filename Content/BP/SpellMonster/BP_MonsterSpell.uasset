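; BP_MonsterSpell is a short-lived monster spell actor that snaps a pair of jaws, sinks downward and removes itself.
; On BeginPlay the Munch timeline rotates the left and right jaw pivots in opposite directions along a curve.
; A short Delay chained from that timeline's Update starts the SInkDown timeline, which lowers the MOV component, then destroys the actor when finished.
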(event EventBeginPlay
  (bind _munchcurve (Timeline|Munch Play)
    (:Update
      (Transformation|SetRelativeRotation (Variables|Default|GetLeftJaw_ROT) (Math|Rotator|Lerp(Rotator) "90.000000, 0, 0" "0, 0, 0" _munchcurve) false false)
      (Transformation|SetRelativeRotation (Variables|Default|GetRightJaw_ROT) (Math|Rotator|Lerp(Rotator) "0.000000, 0, 0" "90.000000,0.000000,0.000000" _munchcurve) false false)
      (Utilities|FlowControl|Delay 0.35)
      (bind _sinkingdowncurve (Timeline|SInkDown Play)
        (:Update
          (Transformation|SetRelativeLocation (Variables|Default|GetMOV) (Math|Vector|Lerp(Vector) "0, 0, 0" "0, 0,-180.000000" _sinkingdowncurve) false false))
        (:Finished
          (Actor|DestroyActor))))))

(fn ConstructionScript)