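; BP_GeneralLightManager finds the BP_LightProps actors belonging to a level number and tracks how many lights remain.
; GetAllLightsByLevelNumber filters all placed light props by LevelNumber into a set and stores its size as the remaining count.
; LightGetsDestroyed decrements that count and prints a warning if it drops below zero, indicating mistagged lights.
; BeginPlay runs a debug test that prints the names of level 1 lights.
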(event EventBeginPlay
  ;[1 1 1] Debug test
  (bind _lights_bp_array (CallFunction|GetAllLightsbyLevelNumber 1))
  (bind _result (Utilities|Set|ToArray _lights_bp_array))
  (for _array_element _result
    (Development|PrintString (Utilities|GetDisplayName _array_element))))

(event Collision|EventActorBeginOverlap
  (params (OtherActor :type Actor%20Object%20Reference)))

(event EventTick
  (params (DeltaSeconds :type Float%20%28single-precision%29)))

(fn ConstructionScript)

(fn GetAllLightsbyLevelNumber
  (params (LevelToSearch :type Integer))
  (Variables|Default|SetTemp_LightArray (Utilities|Set|MakeSet 0))
  (bind _outactors (Actor|GetAllActorsOfClass "/Game/BP/Lights/BP_LightProps.BP_LightProps_C"))
  ;[1 1 1] For each Light found
  (for _array_element _outactors
    ;[1 1 1] if in the right levle
    (if (== (Variables|/Game/BP/Lights/BP_LightProps.BP_LightProps_C|GetLevelNumber _array_element) LevelToSearch)
      ;[1 1 1] Add to the temp List
      (Utilities|Set|Add (Variables|Default|GetTemp_LightArray) _array_element)))
  (Variables|Default|SetNumberOfLightsLeft (Utilities|Set|Length (Variables|Default|GetTemp_LightArray)))
  (return (Variables|Default|GetTemp_LightArray)))

(fn LightGetsDestroyed
  (bind _result (Math|Integer|DecrementInt (Variables|Default|GetNumberOfLightsLeft))
    (:%20%20
      (if (< _result 0)
        (Development|PrintString "NUMBER OF LIGHTS REMAINING < 1. 
WE DESTROYED MORE LIGHTS THAN THERE ARE IN THE LEVEL.  
SOME LIGHTS DIDN'T HAVE THE RIGHT LEVEL NUMBER" true true "(R=0.000000,G=0.660000,B=1.000000,A=1.000000)" 5.0)))))