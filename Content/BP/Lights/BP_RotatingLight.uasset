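; Rotating light actor that sweeps back and forth in yaw around its starting rotation, pausing at each end.
; BeginPlay records the starting yaw; Tick calls RotateOnce to turn by direction, speed and delta time while the pause timer is below zero.
; Passing the maximum offset either way flips the direction and calls ResetTimer, and Tick counts the pause down before rotation resumes.
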(event EventBeginPlay
  (Variables|Default|SetcurrentDirection 1)
  (Variables|Default|SetStartingRotation (.yaw (Transformation|GetActorRotation)))
  (|CallParentFunction))

(event Collision|EventActorBeginOverlap
  (params (OtherActor :type Actor%20Object%20Reference))
  (|CallParentFunction OtherActor) ; This node is disabled and will not be called.\nDrag off pins to build functionality.
)

(event EventTick
  (params (DeltaSeconds :type Float%20%28single-precision%29))
  (bind _returnvalue (Transformation|GetActorRotation))
  (bind _startingrotation (Variables|Default|GetStartingRotation))
  (bind _maximumrotationfromdefault (Variables|Default|GetMaximumRotationFromDefault))
  ;[1 1 1] Only rotate if the PauseTimer is at 0
  (if (< (Variables|Default|GetcurrentTimer) 0.0)
    (CallFunction|RotateOnce DeltaSeconds)
    ;[1 1 1] Change Direction if too far
    (if (> (.yaw _returnvalue) (+ _startingrotation _maximumrotationfromdefault))
      (Variables|Default|SetcurrentDirection -1)
      ;[1 1 1] pause for a few seconds before rotating again
      (CallFunction|ResetTimer :!label _label)
      (elif (< (.yaw _returnvalue) (- _startingrotation _maximumrotationfromdefault))
        (Variables|Default|SetcurrentDirection 1)
        (goto _label)
        (else
          _)))
    (else
      ;[1 1 1] Timer -= Time.deltaTime
      (Variables|Default|SetcurrentTimer (- (Variables|Default|GetcurrentTimer) DeltaSeconds))))
  (|CallParentFunction DeltaSeconds))

(fn ConstructionScript
  (|CallParentFunction))

(fn RotateOnce
  (params (DeltaTime :type Float%20%28double-precision%29))
  (bind _returnvalue (Transformation|GetActorRotation))
  (Transformation|SetActorRotation (Math|Rotator|MakeRotator (.roll _returnvalue) (.pitch _returnvalue) (+ (.yaw _returnvalue) (* (Variables|Default|GetcurrentDirection) (Variables|Default|GetRotationSpeed) DeltaTime)))))

(fn ResetTimer
  (Variables|Default|SetcurrentTimer (Variables|Default|GetPauseTimerBetweenDirections)))