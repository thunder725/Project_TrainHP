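; Stealth enemy that patrols between two locations, shoots at the player on sight and investigates perceived stimuli.
; PawnSensing counts the player as seen only when lit and out of shadow, then turns to face them and fires rate-limited projectiles.
; A retriggerable delay clears sight and resumes patrol, while AIPerception sends the enemy to the stimulus location before patrolling again.
; Player overlap with the light collider opens a hard-coded level.
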(event OnSeePawn(PawnSensing)
  (params (Pawn :type Pawn%20Object%20Reference))
  ;[1 0.4704 0.3401] PawnSensing
  (bind _asbp_first_person_character (Utilities|Casting|CastToBP_FirstPersonCharacter Pawn))
  (Class|NavMovementComponent|StopActiveMovement (Variables|Character|GetCharacterMovement))
  (if (and (not (Variables|/Game/FirstPerson/Blueprints/BP_FirstPersonCharacter.BP_FirstPersonCharacter_C|GetIsShadowPOV _asbp_first_person_character)) (Variables|/Game/FirstPerson/Blueprints/BP_FirstPersonCharacter.BP_FirstPersonCharacter_C|GetIsInLight _asbp_first_person_character))
    (Utilities|FlowControl|Sequence
      (:then_0
        (Variables|Default|SetCanSeePlayer? (Utilities|IsValid Pawn))
        (Variables|Default|SetPatrolStarted? false)
        (Utilities|FlowControl|Sequence
          (:then_0
            ;[1 0.7093 0.3181] Facing the player
            (Transformation|SetActorRotation (Math|Rotator|MakeRotator 0.0 0.0 (.yaw (Math|Rotator|FindLookatRotation (Transformation|GetActorLocation) (Transformation|GetActorLocation _asbp_first_person_character))))))
          (:then_1
            ;[0.8281 0.5168 0.2646] Projectile
            (if (Variables|Default|GetSpawnProjectile)
              (bind _returnvalue (Game|SpawnActorfromClass "/Game/FirstPerson/Blueprints/BP_FirstPersonProjectile.BP_FirstPersonProjectile_C" (Transformation|GetWorldTransform (Variables|Default|GetProjectileSpawnLocation)) "Undefined" 0 0))
              (Physics|AddImpulse (Variables|/Game/FirstPerson/Blueprints/BP_FirstPersonProjectile.BP_FirstPersonProjectile_C|GetSphere _returnvalue) (* (Math|Vector|GetForwardVector (Variables|Default|GetCube)) (Variables|Default|GetShootAmount)) "None" true)
              (Variables|Default|SetSpawnProjectile false)
              (Utilities|FlowControl|Delay 3.0)
              (Variables|Default|SetSpawnProjectile true)))))
      (:then_1
        (Utilities|FlowControl|RetriggerableDelay 0.6)
        (Variables|Default|SetCanSeePlayer? false)
        (CallFunction|Patrol)))))

(event OnTargetPerceptionUpdated(AIPerception)
  (params (Actor :type Actor%20Object%20Reference) (Stimulus :type AI%20Stimulus%20Structure))
  (bind (_age _expirationage _strength _stimuluslocation _receiverlocation _tag _bsuccessfullysensed) (Utilities|Struct|BreakAIStimulus Stimulus))
  ;[1 0.8296 0.403] InvestigateLight
  (Class|NavMovementComponent|StopActiveMovement (Variables|Character|GetCharacterMovement))
  (Variables|Default|SetPatrolStarted? false)
  (Utilities|Casting|CastToBP_FirstPersonCharacter Actor)
  (if _bsuccessfullysensed
    (Variables|Default|SetInvestigating? true)
    (AI|AIMoveTo self _stimuluslocation 0 3e+02 false
      (:OnSuccess
        _)
      (:OnFail
        _))
    (Utilities|FlowControl|Delay 1.0)
    (Variables|Default|SetInvestigating? false)
    (CallFunction|Patrol)))

(event OnComponentBeginOverlap(Light_Collider)
  (params (OverlappedComponent :type Primitive%20Component%20Object%20Reference) (OtherActor :type Actor%20Object%20Reference) (OtherComp :type Primitive%20Component%20Object%20Reference) (OtherBodyIndex :type Integer) (bFromSweep :type Boolean) (SweepResult :type Hit%20Result%20Structure%20%28by%20ref%29))
  ;[1 1 1] Kill Player
  (Utilities|Casting|CastToBP_FirstPersonCharacter OtherActor)
  (Game|OpenLevel(byName) "LevelBuilding_Leo"))

(event Custom|Patrol
  (bind _location1 (Variables|Default|GetLocation1))
  (bind _location2 (Variables|Default|GetLocation2))
  ;[1 0.3495 0.3177] Patrol
  (if (not (Variables|Default|GetCanSeePlayer?))
    (Variables|Default|SetPatrolStarted? true)
    (Transformation|SetActorRotation (Math|Rotator|MakeRotator 0.0 0.0 (.yaw (Math|Rotator|FindLookatRotation (Transformation|GetActorLocation) _location1))))
    (AI|Navigation|SimpleMovetoLocation (Pawn|GetController) _location1 :!label _label)
    (Variables|Default|SetPatrolStarted? false)
    (Utilities|FlowControl|Delay 5.0)
    (if (not (Variables|Default|GetCanSeePlayer?))
      (Transformation|SetActorRotation (Math|Rotator|MakeRotator 0.0 0.0 (.yaw (Math|Rotator|FindLookatRotation (Transformation|GetActorLocation) _location2))))
      (AI|Navigation|SimpleMovetoLocation (Pawn|GetController) _location2)
      (Variables|Default|SetPatrolStarted? false)
      (Utilities|FlowControl|Delay 5.0)
      (if (not (Variables|Default|GetCanSeePlayer?))
        (goto _label)))))

(event EventBeginPlay
  ;[1 0.3495 0.3177] Patrol
  (CallFunction|Patrol))

(fn ConstructionScript)